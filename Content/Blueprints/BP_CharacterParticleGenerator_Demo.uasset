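; BP_CharacterParticleGenerator_Demo gathers socket data from its Mesh, with no particle logic in the graphs shown.
; On BeginPlay, FetchSocketRawData iterates all socket names, appending location, rotation and bone name to three arrays, which it returns.
; SocketNames receives bone names rather than socket names.
; The return sits inside the loop body, so only the first socket is recorded per call.
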(event `self.ReceiveBeginPlay`
  (`self.FetchSocketRawData`))

(fn `FetchSocketRawData`
  (returns (SocketNames :type "Array of Name") (SocketRotations :type "Array of Rotator Structure") (SocketLocations :type "Array of Vector Structure"))
  (for _array_element (`SceneComponent.GetAllSocketNames` (`self.Mesh`))
    (`KismetArrayLibrary.Array_Add` (`self.SocketLocations`) (`SceneComponent.GetSocketLocation` (`self.Mesh`) _array_element))
    (`KismetArrayLibrary.Array_Add` (`self.SocketRotations`) (`SceneComponent.GetSocketRotation` (`self.Mesh`) _array_element))
    (`KismetArrayLibrary.Array_Add` (`self.SocketNames`) (`SkinnedMeshComponent.GetSocketBoneName` (`self.Mesh`) _array_element))
    (return (`self.SocketNames`) (`self.SocketRotations`) (`self.SocketLocations`))))

(fn `UserConstructionScript`)