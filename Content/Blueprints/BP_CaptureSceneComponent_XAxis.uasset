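; X-axis scene capture Blueprint that streams stored frame messages to an MQTT broker.
; BeginPlay connects the level's MqttActor to the broker as the buffer adapter client.
; MessageStored sets the frame rate limit and calls PublishFrame, which, when enabled, sends time plus wrapped positive-X yaw to "bufferTime".
; Frame data goes to "frameData" at higher QoS only after that publish succeeds.
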(event `self.ReceiveBeginPlay`
  (bind _mqttclient (`self.MQTTClient`))
  (set `self.NegativeXRotation` (struct))
  (bind _outactors (`GameplayStatics.GetAllActorsOfClass` "/Script/BPMqtt.MqttActor"))
  (for _array_element _outactors
    (set `self.MQTTClient` _array_element)
    (`MqttActor.CreateClient` _mqttclient "bufferAdapter" (`self.BrokerIPAddress`) 1883 "MQTT_TCP")
    (bind _returnvalue (`MqttActor.Connect` _mqttclient 5 true "" ""))
    (switch `EMqttCode` _returnvalue
      (:`MQTT_SUCCESS`
        (`KismetSystemLibrary.PrintString` "Connected to MQTT")))))

(event `self.MessageStored`
  (`KismetSystemLibrary.PrintString` "Event Message Stored" false false)
  (set `self.frameRateLimit` 3)
  (`self.PublishFrame` (`self.FrameMessage`)))

(event `PublishFrame`
  (params (Message :type "String (by ref)"))
  (bind _mqttclient (`self.MQTTClient`))
  (bind _returnvalue (`KismetStringLibrary.Concat_StrStr` (`self.TimeMessage`) "," (`KismetStringLibrary.Conv_DoubleToString` (mod (.yaw (`self.PositiveXRotation`)) 360.0))))
  (if (`self.PublishMessage`)
    (if true
      (bind _returnvalue_2 (`MqttActor.Publish` _mqttclient "bufferTime" _returnvalue 1))
      (switch `EMqttCode` _returnvalue_2
        (:`MQTT_SUCCESS`
          (`KismetSystemLibrary.PrintString` _returnvalue false false)
          (bind _returnvalue_3 (`MqttActor.Publish` _mqttclient "frameData" Message 2))
          (switch `EMqttCode` _returnvalue_3
            (:`MQTT_SUCCESS`
              (`KismetSystemLibrary.PrintString` Message false false))))
        (:`MQTT_FAIL`
          (`KismetSystemLibrary.PrintString` "Failed to publish time" :!label _label))
        (:`MQTT_DISCONNECTING`
          (goto _label))))))

(fn `UserConstructionScript`)